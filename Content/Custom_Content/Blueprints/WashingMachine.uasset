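; Interactive washing machine that the player switches on and off with R while inside its trigger volume.
; Trigger overlap enables and disables input, and each press toggles the audio component's active state.
; R also starts or stops the WashingMovement timeline, which offsets the Washer component's relative location and sets IsWashing on each update.
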(event OnComponentBeginOverlap(TriggerEnter)
  (params (OverlappedComponent :type Primitive%20Component%20Object%20Reference) (OtherActor :type Actor%20Object%20Reference) (OtherComp :type Primitive%20Component%20Object%20Reference) (OtherBodyIndex :type Integer) (bFromSweep :type Boolean) (SweepResult :type Hit%20Result%20Structure%20%28by%20ref%29))
  (Input|EnableInput (Game|GetPlayerController 0)))

(event OnComponentEndOverlap(TriggerEnter)
  (params (OverlappedComponent :type Primitive%20Component%20Object%20Reference) (OtherActor :type Actor%20Object%20Reference) (OtherComp :type Primitive%20Component%20Object%20Reference) (OtherBodyIndex :type Integer))
  (Input|DisableInput (Game|GetPlayerController 0)))

(event Input|KeyboardEvents|R
  (params (Key :type Key%20Structure :default "AnyKey"))
  (:Pressed
    (Components|Activation|ToggleActive (Variables|Default|GetAudio))
    (if (Variables|Default|GetisWashing)
      (Variables|Default|SetisWashing false)
      (bind _washermovement (Timeline|WashingMovement Stop)
        (:Update
          (Transformation|SetRelativeLocation (Variables|Default|GetWasher) (* _washermovement 5.0) false false)
          (Variables|Default|SetisWashing true)))
      (else
        (Timeline|WashingMovement PlayFromStart)))))

(fn ConstructionScript)