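; Interactive wardrobe actor with two doors that the player opens and closes independently while nearby.
; A Box overlap enables input from player controller 0 on entry and disables it on exit, without filtering the overlapping actor.
; Q toggles LeftDoor and E toggles RightDoor, using MoveComponentTo between hardcoded relative transforms.
; The state flags are named opposite to their doors: ROpen tracks LeftDoor and LOpen tracks RightDoor.
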(event OnComponentBeginOverlap(Box)
  (params (OverlappedComponent :type Primitive%20Component%20Object%20Reference) (OtherActor :type Actor%20Object%20Reference) (OtherComp :type Primitive%20Component%20Object%20Reference) (OtherBodyIndex :type Integer) (bFromSweep :type Boolean) (SweepResult :type Hit%20Result%20Structure%20%28by%20ref%29))
  (Input|EnableInput (Game|GetPlayerController 0)))

(event OnComponentEndOverlap(Box)
  (params (OverlappedComponent :type Primitive%20Component%20Object%20Reference) (OtherActor :type Actor%20Object%20Reference) (OtherComp :type Primitive%20Component%20Object%20Reference) (OtherBodyIndex :type Integer))
  (Input|DisableInput (Game|GetPlayerController 0)))

(event Input|KeyboardEvents|Q
  (params (Key :type Key%20Structure))
  (bind _leftdoor (Variables|Default|GetLeftDoor))
  (:Pressed
    (if (Variables|Default|GetROpen)
      (Components|MoveComponentTo _leftdoor "-25.000000,1050.000000, 0" "0, 0, 0" false false 0.2 false)
      (Variables|Default|SetROpen false)
      (else
        (Components|MoveComponentTo _leftdoor "-62.000000,1380.000000, 0" "0,135.000000, 0" false false 0.2 false)
        (Variables|Default|SetROpen true)))))

(event Input|KeyboardEvents|E
  (params (Key :type Key%20Structure))
  (bind _rightdoor (Variables|Default|GetRightDoor))
  (:Pressed
    (if (Variables|Default|GetLOpen)
      (Components|MoveComponentTo _rightdoor "25.000000,1050.000000, 0" "0, 0, 0" false false 0.2 false)
      (Variables|Default|SetLOpen false)
      (else
        (Components|MoveComponentTo _rightdoor "62.000000,1380.000000, 0" "0,-135.000000, 0" false false 0.2 false)
        (Variables|Default|SetLOpen true)))))

(fn ConstructionScript)